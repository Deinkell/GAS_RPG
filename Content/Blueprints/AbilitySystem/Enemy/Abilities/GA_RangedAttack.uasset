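; Enemy ranged attack gameplay ability that fires a projectile at the avatar's current combat target.
; On activation it turns the avatar toward the target and plays a random tagged attack montage.
; A gameplay event matching the montage tag re-reads the target location, spawns the projectile from the tagged socket with optional pitch override, then ends the ability.
; Montage completion, interruption or cancellation also ends the ability.
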(event `self.K2_ActivateAbility`
  (bind _returnvalue (`self.GetAvatarActorFromActorInfo`))
  (bind _returnvalue_2 (message `EnemyInterface.GetCombatTarget` _returnvalue))
  (bind _ascombat_interface (cast `CombatInterface` _returnvalue))
  (`CombatInterface.UpdateFacingTarget` _ascombat_interface (`Actor.K2_GetActorLocation` _returnvalue_2))
  (bind _returnvalue_3 (`CombatInterface.GetAttackMontages` _ascombat_interface))
  (bind _output_get (set `self.TaggedMontage` (`self.GetRandomTaggedMontageFromArray` _returnvalue_3)))
  (bind (_montage _montagetag _sockettag) (break `TaggedMontage` _output_get))
  (`AbilityTask_PlayMontageAndWait.CreatePlayMontageAndWaitProxy` "None" _montage 1.0 "None" false
    (:`then`
      (`AbilityTask_WaitGameplayEvent.WaitGameplayEvent` _montagetag null true
        (:`EventReceived`
          (bind _returnvalue_4 (message `EnemyInterface.GetCombatTarget` (`self.GetAvatarActorFromActorInfo`)))
          (`self.SpawnProjectile` (`Actor.K2_GetActorLocation` _returnvalue_4) _sockettag (`self.ShouldOverridePitch`) (`self.PitchOverride`))
          (`self.K2_EndAbility`))))
    (:`OnCompleted`
      (`self.K2_EndAbility` :!label _label))
    (:`OnInterrupted`
      (goto _label))
    (:`OnCancelled`
      (goto _label))))