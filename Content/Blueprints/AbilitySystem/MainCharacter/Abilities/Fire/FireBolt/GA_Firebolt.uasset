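; Gameplay ability for the main character's Firebolt, which fires a projectile at the point under the mouse.
; It reads the target location, turns the avatar toward it through the combat interface, then commits if allowed and plays a katana montage.
; A montage gameplay event times the projectile spawn from the weapon socket.
; Controller-driven rotation is suspended during the cast and restored with control rotation synced to the actor on release or montage end.
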(event `self.K2_ActivateAbility`
  (bind (_asynctaskproxy _datahandle) (`TargetDataUnderMouse.CreateTargetDataUnderMouse`)
    (:`ValidData`
      (set `self.ProjectileTargetLocation` (`.Location` (`GameplayStatics.BreakHitResult` (`AbilitySystemBlueprintLibrary.GetHitResultFromTargetData` _datahandle))))
      (bind _ascombat_interface (cast `CombatInterface` (`self.GetAvatarActorFromActorInfo`)))
      (`CombatInterface.UpdateFacingTarget` _ascombat_interface (`self.ProjectileTargetLocation`))
      (bind _returnvalue (`self.CanFirebolt`))
      (if _returnvalue
        (`self.K2_CommitAbility`)
        (bind _asbp_main_character (cast `/Game/Blueprints/Character/MainCharacter/BP_MainCharacter` (`self.GetAvatarActorFromActorInfo`)))
        (bind _output_get (set `self.BP Main Character` _asbp_main_character))
        (`MainCharacter.SetControllerRotationAndDesiredRotation` _output_get false)
        (`AbilityTask_PlayMontageAndWait.CreatePlayMontageAndWaitProxy` "None" "/Game/Blueprints/Character/MainCharacter/Animation_Montage/AM_Katana_Firebolt.AM_Katana_Firebolt" 1.0 "None" false
          (:`then`
            (`AbilityTask_WaitGameplayEvent.WaitGameplayEvent` (struct :`TagName` "Event.Montage.Firebolt") null
              (:`EventReceived`
                (`self.SpawnProjectile` (`self.ProjectileTargetLocation`) (`BlueprintGameplayTagLibrary.MakeLiteralGameplayTag` (struct :`TagName` "CombatSocket.Weapon")))
                (bind _returnvalue_2 (`MainCharacter.GetMPPlayerController` (`self.BP Main Character`)))
                (`Controller.SetControlRotation` _returnvalue_2 (`Actor.K2_GetActorRotation` (`self.BP Main Character`)))
                (`MainCharacter.SetControllerRotationAndDesiredRotation` (`self.BP Main Character`) true))))
          (:`OnCompleted`
            (`self.K2_EndAbility` :!label _label)
            (bind _returnvalue_3 (`MainCharacter.GetMPPlayerController` (`self.BP Main Character`)))
            (`Controller.SetControlRotation` _returnvalue_3 (`Actor.K2_GetActorRotation` (`self.BP Main Character`)))
            (`MainCharacter.SetControllerRotationAndDesiredRotation` (`self.BP Main Character`) true))
          (:`OnBlendOut`
            (goto _label))
          (:`OnInterrupted`
            (goto _label))
          (:`OnCancelled`
            (goto _label)))
        (else
          (`self.K2_EndAbility`))))))